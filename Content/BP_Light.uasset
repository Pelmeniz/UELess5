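; BP_Light is a light Blueprint that blinks its PointLight a set number of times when play begins, then leaves it off.
; BeginPlay hides the light, then a DoN node capped by IndexFlashes drives a loop that turns it on and off with a TimeFlashes delay before each change.
; The loop wires back into DoN without a reset, so flashing ends once the count is used up.
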(event EventBeginPlay
  (Rendering|SetVisibility (Variables|Default|GetPointLight) false false)
  (Utilities|FlowControl|DoN (Variables|Default|GetIndex%20Flashes) :!label _label
    (:Exit
      (Utilities|FlowControl|Delay (Variables|Default|GetTime%20Flashes))
      (Rendering|SetVisibility (Variables|Default|GetPointLight) true false)
      (Utilities|FlowControl|Delay (Variables|Default|GetTime%20Flashes))
      (Rendering|SetVisibility (Variables|Default|GetPointLight) false false)
      (goto _label))))

(fn ConstructionScript)